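; Base character Blueprint that handles damage reactions, ragdoll, camera-facing toggles and weapon cleanup on EndPlay.
; Unless a state check blocks it, damage updates StatusComponent and StateComponent, passes the causer's location to ABP_General and flashes the mesh red through dynamic materials created at BeginPlay.
; It then plays a directional hit or death montage from WeaponComponent's current data asset.
; Helpers enable ragdoll physics with a timer, switch rotation modes and offset the camera's Y.
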(event `self.ReceiveBeginPlay`
  (for (_array_element _array_index) (`MeshComponent.GetMaterials` (`self.Mesh`))
    (bind _returnvalue (`KismetMaterialLibrary.CreateDynamicMaterialInstance` _array_element))
    (`PrimitiveComponent.SetMaterial` (`self.Mesh`) _array_index _returnvalue)))

(event `self.ReceiveAnyDamage`
  (params (Damage :type "Float (single-precision)") (DamageType :type "DamageType Object Reference") (InstigatedBy :type "Controller Object Reference") (DamageCauser :type "Actor Object Reference"))
  (bind _statecomponent (`self.StateComponent`))
  (bind _weaponcomponent (`self.WeaponComponent`))
  (bind _weaponcomponent_2 (`self.WeaponComponent`))
  (bind _returnvalue (`MeshComponent.GetMaterials` (`self.Mesh`)))
  (bind (_output_montage _output_playrate) (break `/Game/DataAsset/Structs/FMontage` (`|GetArrayItem` (`/Game/Weapons/BluePrints/BP_WeaponData.DeathMontages` (`/Game/Components/BP_WeaponComponent.CurrentDataAsset` _weaponcomponent)) (`/Game/Components/BP_WeaponComponent.FindCauserDirection` _weaponcomponent DamageCauser))))
  (bind (_output_montage_2 _output_playrate_2) (break `/Game/DataAsset/Structs/FMontage` (`|GetArrayItem` (`/Game/Weapons/BluePrints/BP_WeaponData.HitMontages` (`/Game/Components/BP_WeaponComponent.CurrentDataAsset` _weaponcomponent_2)) (`/Game/Components/BP_WeaponComponent.FindCauserDirection` _weaponcomponent_2 DamageCauser))))
  (if (not (`/Game/Components/BP_StateComponent.IsMyState` (`self.StateComponent`) "NewEnumerator5"))
    (`|ExecutionSequence`
      (:`then_0`
        (bind _currenthp (`/Game/Components/BP_StatusComponent.OnDamaged` (`self.StatusComponent`) Damage))
        (if (<= _currenthp 0.0)
          (set `/Game/Components/BP_StateComponent.MyState` "NewEnumerator2" _statecomponent)
          (else
            (set `/Game/Components/BP_StateComponent.MyState` "NewEnumerator1" _statecomponent))))
      (:`then_1`
        (bind _asabp_general (cast `/Game/Animations/AnimInstance/ABP_General` (`SkeletalMeshComponent.GetAnimInstance` (`self.Mesh`))))
        (set `/Game/Animations/AnimInstance/ABP_General.DamageCauserLocation` (`self.K2_GetActorLocation` DamageCauser) _asabp_general))
      (:`then_2`
        (for _array_element _returnvalue
          (bind `_as머티리얼_인스턴스_다이내믹` (cast `MaterialInstanceDynamic` _array_element))
          (`MaterialInstanceDynamic.SetVectorParameterValue` `_as머티리얼_인스턴스_다이내믹` "Color" (struct :`R` 1.0 :`A` 1.0)))
        (`KismetSystemLibrary.Delay` 0.2)
        (for _array_element_2 _returnvalue
          (bind `_as머티리얼_인스턴스_다이내믹_2` (cast `MaterialInstanceDynamic` _array_element_2))
          (`MaterialInstanceDynamic.SetVectorParameterValue` `_as머티리얼_인스턴스_다이내믹_2` "Color" (struct :`R` 1.0 :`G` 1.0 :`B` 1.0 :`A` 1.0))))
      (:`then_3`
        (if (`/Game/Components/BP_StateComponent.isHitted` (`self.StateComponent`) "NewEnumerator2")
          (`/Engine/EditorBlueprintResources/StandardMacros.IsValid` _output_montage
            (:`Is Valid`
              (`self.PlayAnimMontage` _output_montage _output_playrate)))
          (else
            (`/Engine/EditorBlueprintResources/StandardMacros.IsValid` _output_montage_2
              (:`Is Valid`
                (`self.PlayAnimMontage` _output_montage_2 _output_playrate_2)))))))))

(event `self.ReceiveEndPlay`
  (params (EndPlayReason :type "EEndPlayReason Enum" :default "Destroyed"))
  (`/Game/Components/BP_WeaponComponent.DestroyAllWeapons` (`self.WeaponComponent`)))

(fn `CameraLock`
  (params (CameraHold :type Boolean))
  (set `CharacterMovementComponent.bOrientRotationToMovement` (not CameraHold) (`self.CharacterMovement`))
  (set `self.bUseControllerRotationYaw` CameraHold))

(fn `CameraUnlock`
  (params (CameraHold :type Boolean))
  (set `CharacterMovementComponent.bOrientRotationToMovement` CameraHold (`self.CharacterMovement`))
  (set `self.bUseControllerRotationYaw` (not CameraHold)))

(fn `SetCameraRelativeYpos`
  (params (Y :type "Float (double-precision)"))
  (bind _returnvalue (`self.GetComponentByClass` "/Script/Engine.CameraComponent"))
  (`/Engine/EditorBlueprintResources/StandardMacros.IsValid` _returnvalue
    (:`Is Valid`
      (`SceneComponent.K2_SetRelativeLocation` _returnvalue (`KismetMathLibrary.MakeVector` 0.0 Y) false false))))

(fn `SetRegdoll`
  (bind _mesh (`self.Mesh`))
  (`PrimitiveComponent.SetSimulatePhysics` _mesh true)
  (`PrimitiveComponent.SetCollisionProfileName` _mesh "Ragdoll" true)
  (`PrimitiveComponent.SetCollisionProfileName` (`self.CapsuleComponent`) "IgnoreOnlyPawn" true)
  (`KismetSystemLibrary.K2_SetTimerDelegate` (`|CreateDelegate` :!event `K2_DestroyActor`) 3.0))

(fn `UserConstructionScript`)