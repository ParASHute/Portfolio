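; BP_Link is the player character Blueprint for Link, handling movement, camera look, jumping and sword selection.
; BeginPlay sets walk speed, then runs the Move graph, which registers general and combat Enhanced Input mapping contexts.
; Move input follows control yaw, while raw Shift and Alt keys switch MaxWalkSpeed for sprint and slow walk.
; The sword action delegates to WeaponComponent; initial speed equals sprint speed until either key is released.
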(event `self.ReceiveBeginPlay`
  (`|ExecutionSequence`
    (:`then_0`
      (set `CharacterMovementComponent.MaxWalkSpeed` 750.0 (`self.CharacterMovement`)))
    (:`then_1`
      (bind `_as플레이어_컨트롤러` (cast `PlayerController` (`self.GetController`)))
      (bind _returnvalue (pcsubsystem `EnhancedInputLocalPlayerSubsystem` `_as플레이어_컨트롤러`))
      (`EnhancedInputSubsystemInterface.AddMappingContext` _returnvalue "/Game/Characters/Link/Input/General/IMC_General.IMC_General" 0 (struct))
      (`EnhancedInputSubsystemInterface.AddMappingContext` _returnvalue "/Game/Characters/Link/Input/Combat/IMC_Combat.IMC_Combat" 0 (struct)))))

(event `EnhancedInput|/Game/Characters/Link/Input/General/IA_Move`
  (params (ActionValue :type "Vector2D Structure") (ElapsedSeconds :type "Float (double-precision)") (TriggeredSeconds :type "Float (double-precision)") (InputAction :type "InputAction Object Reference" :default "/Game/Characters/Link/Input/General/IA_Move.IA_Move"))
  (bind (_x _y) (`KismetMathLibrary.BreakVector2D` ActionValue))
  (bind (_returnvalue_roll _returnvalue_pitch _returnvalue_yaw) (`KismetMathLibrary.BreakRotator` (`self.GetControlRotation`)))
  (bind _returnvalue (`KismetMathLibrary.MakeRotator` 0.0 0.0 _returnvalue_yaw))
  (:`Triggered`
    (`self.AddMovementInput` (`KismetMathLibrary.GetRightVector` _returnvalue) _x)
    (`self.AddMovementInput` (`KismetMathLibrary.GetForwardVector` _returnvalue) _y)))

(event `EnhancedInput|/Game/Characters/Link/Input/General/IA_View`
  (params (ActionValue :type "Vector2D Structure") (ElapsedSeconds :type "Float (double-precision)") (TriggeredSeconds :type "Float (double-precision)") (InputAction :type "InputAction Object Reference" :default "/Game/Characters/Link/Input/General/IA_View.IA_View"))
  (:`Triggered`
    (`self.AddControllerYawInput` ActionValue_X)
    (`self.AddControllerPitchInput` ActionValue_Y)))

(event `Key|LeftShift`
  (params (Key :type "Key Structure"))
  (bind _charactermovement (`self.CharacterMovement`))
  (:`Pressed`
    (set `CharacterMovementComponent.MaxWalkSpeed` 750.0 _charactermovement))
  (:`Released`
    (set `CharacterMovementComponent.MaxWalkSpeed` 500.0 _charactermovement)))

(event `Key|LeftAlt`
  (params (Key :type "Key Structure"))
  (bind _charactermovement (`self.CharacterMovement`))
  (:`Pressed`
    (set `CharacterMovementComponent.MaxWalkSpeed` 125.0 _charactermovement))
  (:`Released`
    (set `CharacterMovementComponent.MaxWalkSpeed` 500.0 _charactermovement)))

(event `EnhancedInput|/Game/Characters/Link/Input/General/IA_Jump`
  (params (ActionValue :type Boolean) (ElapsedSeconds :type "Float (double-precision)") (TriggeredSeconds :type "Float (double-precision)") (InputAction :type "InputAction Object Reference" :default "/Game/Characters/Link/Input/General/IA_Jump.IA_Jump"))
  (:`Started`
    (`self.Jump`))
  (:`Completed`
    (`self.StopJumping`)))

(event `EnhancedInput|/Game/Characters/Link/Input/Combat/IA_Sword`
  (params (ActionValue :type Boolean) (ElapsedSeconds :type "Float (double-precision)") (TriggeredSeconds :type "Float (double-precision)") (InputAction :type "InputAction Object Reference" :default "/Game/Characters/Link/Input/Combat/IA_Sword.IA_Sword"))
  (:`Triggered`
    (`/Game/Components/BP_WeaponComponent.SelectWeapon` (`self.WeaponComponent`) "NewEnumerator0")))

(fn `UserConstructionScript`
  (`parent.UserConstructionScript`))