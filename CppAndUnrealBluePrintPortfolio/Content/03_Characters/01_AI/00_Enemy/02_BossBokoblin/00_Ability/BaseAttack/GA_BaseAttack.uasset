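; GA_BaseAttack is a base gameplay ability for Boss Bokoblin attacks, with empty activate and end events.
; Its MeleeAttack function spawns a BP_MeleeAttack actor at an offset derived from the owner's transform, with the owner's scale, and initializes it with Radius and Damage.
; GetEnemtChannel is unfinished, only casting the owner to BP_BaseCharacter.
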(fn `GetEnemtChannel`
  (cast `/Game/03_Characters/BP_BaseCharacter` (`self.GetOwningActorFromActorInfo`)))

(fn `MeleeAttack`
  (params (Forward :type "Float (double-precision)"))
  (bind _returnvalue (`self.GetOwningActorFromActorInfo`))
  (bind _returnvalue_2 (`|SpawnActorFromClass` "/Game/02_Equpments/01_Monster/Collision/HitCollision/BP_MeleeAttack.BP_MeleeAttack_C" (`KismetMathLibrary.MakeTransform` (+ (* Forward (.rotation (`Actor.GetTransform` _returnvalue))) (.location (`Actor.GetTransform` _returnvalue))) (struct) (.scale (`Actor.GetTransform` _returnvalue))) "Undefined" "MultiplyWithRoot" _returnvalue (`Actor.Instigator` _returnvalue)))
  (`/Game/02_Equpments/01_Monster/Collision/HitCollision/BP_HitCollision.OnInit` _returnvalue_2 (`self.Radius`) (`self.Damage`)))