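; GA_JustRush is a Link shield gameplay ability that performs a quick backward dodge and then returns to defence.
; Once committed, it plays the dodge-back montage at increased rate while a constant root motion force pushes Link opposite his facing.
; On blend out, it reactivates the State.Defence ability unless Link's Cancled flag is set, then ends.
; A failed commit, interruption or cancellation ends it directly.
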(event `self.K2_ActivateAbility`
  (bind _returnvalue (`self.K2_CommitAbility`))
  (if _returnvalue
    (`AbilityTask_PlayMontageAndWait.CreatePlayMontageAndWaitProxy` "None" "/Game/00_PlayerAnimation/02_Montage/02_Shield/Dodge/IP_dodge_back_Montage.IP_dodge_back_Montage" 2.0
      (:`then`
        (bind _asbp_link (cast `/Game/03_Characters/00_Link/BP_Link` (`self.GetOwningActorFromActorInfo`)))
        (`AbilityTask_ApplyRootMotionConstantForce.ApplyRootMotionConstantForce` "None" (* (`Actor.GetActorForwardVector` _asbp_link) -1.0) 150.0 0.8 false null "MaintainLastRootMotionVelocity" (`Actor.GetVelocity` _asbp_link)))
      (:`OnBlendOut`
        (bind _asbp_link_2 (cast `/Game/03_Characters/00_Link/BP_Link` (`self.GetOwningActorFromActorInfo`)))
        (if (not (`/Game/03_Characters/00_Link/BP_Link.Cancled` _asbp_link_2))
          (`AbilitySystemComponent.TryActivateAbilitiesByTag` (`PortfolioCharacter.AbilitySystemComponent` _asbp_link_2) (`BlueprintGameplayTagLibrary.MakeLiteralGameplayTagContainer` (struct :`GameplayTags` (struct :`(TagName` "State.Defence")))) true))
        (`self.K2_EndAbility`))
      (:`OnInterrupted`
        (`self.K2_EndAbility` :!label _label))
      (:`OnCancelled`
        (goto _label)))
    (else
      (`self.K2_EndAbility`))))