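; Gameplay ability that performs Link's shield parry.
; After committing, it plays the parry montage, and ends if the commit fails or the montage is interrupted or cancelled.
; On blend out, it reactivates the State.Defence ability through Link's ability system component unless Link's Cancled flag is set, then ends.
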(event `self.K2_ActivateAbility`
  (bind _returnvalue (`self.K2_CommitAbility`))
  (if _returnvalue
    (`AbilityTask_PlayMontageAndWait.CreatePlayMontageAndWaitProxy` "None" "/Game/00_PlayerAnimation/02_Montage/02_Shield/Parry/IP_parry_Montage.IP_parry_Montage"
      (:`OnBlendOut`
        (bind _asbp_link (cast `/Game/03_Characters/00_Link/BP_Link` (`self.GetOwningActorFromActorInfo`)))
        (if (not (`/Game/03_Characters/00_Link/BP_Link.Cancled` _asbp_link))
          (`AbilitySystemComponent.TryActivateAbilitiesByTag` (`PortfolioCharacter.AbilitySystemComponent` _asbp_link) (`BlueprintGameplayTagLibrary.MakeLiteralGameplayTagContainer` (struct :`GameplayTags` (struct :`(TagName` "State.Defence")))) true))
        (`self.K2_EndAbility`))
      (:`OnInterrupted`
        (`self.K2_EndAbility` :!label _label))
      (:`OnCancelled`
        (goto _label)))
    (else
      (`self.K2_EndAbility`))))