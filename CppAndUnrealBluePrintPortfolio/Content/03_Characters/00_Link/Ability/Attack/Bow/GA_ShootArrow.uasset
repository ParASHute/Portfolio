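; Gameplay ability for Link's bow shot that calls a line-trace function on the equipped bow.
; On activation it commits, gets Link's current weapon as BP_Bow, and passes the bone behind the LineTrace socket to ShootLineBone with a short range.
; The result is only printed before the ability ends, and no arrow is spawned here.
; A failed commit ends the ability, but a failed cast stops without ending it.
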(event `self.K2_ActivateAbility`
  (bind _returnvalue (`self.K2_CommitAbility`))
  (if _returnvalue
    (bind _asbp_link (cast `/Game/03_Characters/00_Link/BP_Link` (`self.GetOwningActorFromActorInfo`)))
    (bind _asbp_bow (cast `/Game/02_Equpments/0_WeaponBluprints/01_Bow/BP_Bow` (`WeaponComponent.CurrentWeapon` (`PortfolioCharacter.WeaponComponent` _asbp_link))))
    (bind _returnvalue_2 (`/Game/02_Equpments/0_WeaponBluprints/01_Bow/BP_Bow.ShootLineBone` _asbp_bow (`SkinnedMeshComponent.GetSocketBoneName` (`BaseWeapon.SkeletalMesh` _asbp_bow) "LineTrace") 200.0))
    (`KismetSystemLibrary.PrintString` (`KismetStringLibrary.Conv_TransformToString` _returnvalue_2))
    (`self.K2_EndAbility`)
    (else
      (`self.K2_EndAbility`))))