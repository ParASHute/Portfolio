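; Gameplay ability for Link's first sword attack, playing the Attack_01 montage and damaging the target of a hit event.
; After committing, it waits for a Hit.Hit1 gameplay event while the montage starts.
; The equipped weapon's damage, scaled to a negative fraction, feeds GE_Damage via SetByCaller, with the target's own ability system applying it to itself.
; The ability ends on montage blend-out, interruption, cancellation or failed commit.
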(event `self.K2_ActivateAbility`
  ;[1 1 1] Death테그가 붙지 않고, State가 ArmedSword일때 실행 할 수 있고
  ; 에택테그의 스택을 쌓지 못하고
  ; 어택이 끝나는 대로 플레이어에게 State.Attack테그가 빠진다
  (bind _returnvalue (`self.K2_CommitAbility`))
  (if _returnvalue
    (`AbilityTask_PlayMontageAndWait.CreatePlayMontageAndWaitProxy` "None" "/Game/00_PlayerAnimation/02_Montage/00_Sword/Attack/Attack_01_Seq_Montage.Attack_01_Seq_Montage"
      (:`then`
        ;[1 1 1] 데이터 에셋에서 무기 공격력받고 배율로 조정
        (bind _asbp_base_character (cast `/Game/03_Characters/BP_BaseCharacter` (`self.GetOwningActorFromActorInfo`)))
        ;[1 1 1] 데미지 넣는 부분
        (bind (_asynctaskproxy _payload) (`AbilityTask_WaitGameplayEvent.WaitGameplayEvent` (struct :`TagName` "Hit.Hit1") null) ; 테그 이벤트 발송시 뒤에것들 실행
          (:`EventReceived`
            (bind _returnvalue_2 (`AbilitySystemBlueprintLibrary.GetAbilitySystemComponent` (`.Target` (break `GameplayEventData` _payload))))
            (bind _returnvalue_3 (`AbilitySystemBlueprintLibrary.AssignTagSetByCallerMagnitude` (`AbilitySystemComponent.MakeOutgoingSpec` :`self` _returnvalue_2 :`GameplayEffectClass` "/Game/03_Characters/00_Link/Ability/GE_Damage.GE_Damage_C" :`Level` 1.0) (struct :`TagName` "Hit.Hit1") (* (`WeaponData.WeaponDamage` (`WeaponComponent.CurrentWeaponDataAsset` (`PortfolioCharacter.WeaponComponent` _asbp_base_character))) -0.25)))
            (`AbilitySystemComponent.BP_ApplyGameplayEffectSpecToSelf` _returnvalue_2 _returnvalue_3))))
      (:`OnBlendOut`
        (`self.K2_EndAbility` :!label _label))
      (:`OnInterrupted`
        (goto _label))
      (:`OnCancelled`
        (goto _label)))
    (else
      (`self.K2_EndAbility`))))