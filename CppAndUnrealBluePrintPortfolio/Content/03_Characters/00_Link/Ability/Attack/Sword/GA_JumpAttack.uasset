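; GA_JumpAttack is a Gameplay Ability for Link's sword attack while jumping, damaging whatever it hits.
; After commit, it listens for Hit gameplay events and ends when the State.Jump tag is removed.
; Each hit applies GE_Damage to the event target, using SetByCaller to pass a negative quarter of the current weapon data asset's damage.
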(event `self.K2_ActivateAbility`
  (bind _returnvalue (`self.K2_CommitAbility`))
  (if _returnvalue
    (`AbilityTask_WaitGameplayTagRemoved.WaitGameplayTagRemove` (struct :`TagName` "State.Jump") null
      (:`then`
        (bind _asbp_link (cast `/Game/03_Characters/00_Link/BP_Link` (`self.GetOwningActorFromActorInfo`)))
        (bind (_asynctaskproxy _payload) (`AbilityTask_WaitGameplayEvent.WaitGameplayEvent` (struct :`TagName` "Hit") null) ; 테그 이벤트 발송시 뒤에것들 실행
          (:`EventReceived`
            (bind _returnvalue_2 (`AbilitySystemBlueprintLibrary.AssignTagSetByCallerMagnitude` (`self.MakeOutgoingGameplayEffectSpec` "/Game/03_Characters/00_Link/Ability/GE_Damage.GE_Damage_C") (struct :`TagName` "Hit.Hit1") (* (`WeaponData.WeaponDamage` (`WeaponComponent.CurrentWeaponDataAsset` (`PortfolioCharacter.WeaponComponent` _asbp_link))) -0.25)))
            (`AbilitySystemComponent.BP_ApplyGameplayEffectSpecToSelf` (`AbilitySystemBlueprintLibrary.GetAbilitySystemComponent` (`.Target` (break `GameplayEventData` _payload))) _returnvalue_2))))
      (:`Removed`
        (`self.K2_EndAbility`)))
    (else
      (`self.K2_EndAbility`))))