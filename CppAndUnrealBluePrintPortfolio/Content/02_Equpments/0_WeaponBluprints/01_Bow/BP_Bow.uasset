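; Bow weapon Blueprint that handles the aim camera and arrow firing for its owning character.
; Stretch and shoot events play and reverse a timeline that moves the owner's camera.
; SpawnProjectile creates the data asset's projectile without collision, attached to ArrowSocket.
; LanchPorjectile enables overlaps, detaches it, orients it toward a camera trace point, and launches it along control rotation at the data asset's speed.
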(event `Strech`
  (bind (_direction _xpos _ypos _zpos) (`Timeline|SetCameraYPos` :!label _label)
    (:`Update`
      (`PortfolioCharacter.SetCameraRelativePos` (`self.OwnerCharacter`) _xpos _ypos _zpos))))

(event `Shoot`
  (goto _label :!via `Reverse`))

(fn `CameraLineTrace`
  (params (TraceRange :type "Float (double-precision)"))
  (returns (OutputPin :type Boolean) (ReturnValue :type "Vector Structure"))
  (bind _followcamera (`PortfolioCharacter.FollowCamera` (`self.OwnerCharacter`)))
  (bind _returnvalue (`SceneComponent.K2_GetComponentLocation` _followcamera))
  (bind (_outhit _returnvalue_2) (`KismetSystemLibrary.LineTraceSingle` :`Start` _returnvalue :`End` (+ _returnvalue (* TraceRange (`SceneComponent.GetForwardVector` _followcamera))) :`TraceChannel` "TraceTypeQuery4" :`DrawTime` 10000.0))
  (bind (_bblockinghit _binitialoverlap _time _distance _location _impactpoint _normal _impactnormal _physmat _hitactor _hitcomponent _hitbonename _bonename _hititem _elementindex _faceindex _tracestart _traceend) (`GameplayStatics.BreakHitResult` _outhit))
  (return _returnvalue_2 (`KismetMathLibrary.SelectVector` _location _traceend _returnvalue_2)))

(fn `LanchPorjectile`
  (bind _fireprojectile (`self.FireProjectile`))
  (bind _projectilemovement (`BaseProjectile.ProjectileMovement` (`self.FireProjectile`)))
  (`PrimitiveComponent.SetCollisionProfileName` (`BaseProjectile.Capsule` (`self.FireProjectile`)) "OverlapAllDynamic" true)
  (`/Engine/EditorBlueprintResources/StandardMacros.IsValid` (`self.FireProjectile`)
    (:`Is Valid`
      (bind _returnvalue (`self.ShootLineBone` "ArrowSocket" 5000.0))
      (`self.K2_DetachFromActor` _fireprojectile "KeepWorld" "KeepWorld" "KeepWorld")
      (`self.K2_SetActorTransform` _fireprojectile _returnvalue false false)
      (set `ProjectileMovementComponent.bSimulationEnabled` true _projectilemovement)
      (set `MovementComponent.Velocity` (* (`KismetMathLibrary.GetForwardVector` (`Pawn.GetControlRotation` (`self.OwnerCharacter`))) (`WeaponData.ProjectileSpeed` (`self.DataAsset`))) _projectilemovement))))

(fn `ShootLineBone`
  (params (SocketName :type Name) (TraceRange :type "Float (double-precision)"))
  (returns (ReturnValue :type "Transform Structure"))
  (bind _returnvalue (`PortfolioCharacter.GetBone` (`self.OwnerCharacter`) SocketName))
  (bind (_outputpin _returnvalue_2) (`self.CameraLineTrace` TraceRange))
  (bind _location (.location _returnvalue))
  (return (`KismetMathLibrary.MakeTransform` _location (`KismetMathLibrary.FindLookAtRotation` _location _returnvalue_2))))

(fn `SpawnProjectile`
  (bind _projectileclass (`WeaponData.ProjectileClass` (`self.DataAsset`)))
  (if (`KismetSystemLibrary.IsValidClass` _projectileclass)
    (bind _returnvalue (`|SpawnActorFromClass` _projectileclass (`KismetMathLibrary.MakeTransform` (0.0 0.0 0.0)) "Undefined" "MultiplyWithRoot" null (`self.OwnerCharacter`)))
    (bind _output_get (set `self.FireProjectile` _returnvalue))
    (`PrimitiveComponent.SetCollisionProfileName` (`BaseProjectile.StaticMesh` _output_get) "NoCollision" true)
    (`PrimitiveComponent.SetCollisionProfileName` (`BaseProjectile.Capsule` _output_get) "NoCollision" true)
    (set `ProjectileMovementComponent.InitialSpeed` (`WeaponData.ProjectileSpeed` (`self.DataAsset`)) (`BaseProjectile.ProjectileMovement` _output_get))
    (`self.K2_AttachToComponent` _output_get (`self.SkeletalMesh`) "ArrowSocket" "KeepRelative" "KeepRelative" "KeepRelative" true)))

(fn `UserConstructionScript`)