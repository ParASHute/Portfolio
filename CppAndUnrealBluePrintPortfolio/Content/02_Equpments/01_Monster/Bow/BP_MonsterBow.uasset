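; BP_MonsterBow is a monster's longbow weapon that animates its draw, hold and shot and fires projectiles.
; SpawnProjectile creates the data asset's projectile class, sets its speed and attaches it to the mesh's ArrowSocket.
; LanchPorjectile detaches it, aims it at a trace hit or endpoint, then enables its movement.
; Despite its name, CameraLineTrace traces along the skeletal mesh's forward vector rather than from a camera.
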(event `PlayStrechMontage`
  (if (`self.Do`)
    (`SkeletalMeshComponent.PlayAnimation` (`self.SkeletalMesh`) "/Game/01_MonsterAnimation/05_Sequence/Bokoblin02/Bow/AS_Longbow3_Strech_L.AS_Longbow3_Strech_L" false)))

(event `PlayLoopMontage`
  (`SkeletalMeshComponent.PlayAnimation` (`self.SkeletalMesh`) "/Game/01_MonsterAnimation/05_Sequence/Bokoblin02/Bow/AS_Longbow3_Loop_L.AS_Longbow3_Loop_L" false))

(event `PlayShootMontage`
  (`SkeletalMeshComponent.PlayAnimation` (`self.SkeletalMesh`) "/Game/01_MonsterAnimation/05_Sequence/Bokoblin02/Bow/AS_Longbow3_Shot_L.AS_Longbow3_Shot_L" false))

(fn `CameraLineTrace`
  (params (TraceRange :type "Float (double-precision)"))
  (returns (ReturnValue :type "Vector Structure"))
  (locals (NewLocalVar :type "Vector Structure" :default (0.0 0.0 0.0)))
  (bind _skeletalmesh (`self.SkeletalMesh`))
  (bind _returnvalue (`SceneComponent.GetSocketLocation` _skeletalmesh "None"))
  (bind (_outhit _returnvalue_2) (`KismetSystemLibrary.LineTraceSingle` :`Start` _returnvalue :`End` (+ _returnvalue (* TraceRange (`SceneComponent.GetForwardVector` _skeletalmesh))) :`TraceChannel` "TraceTypeQuery4" :`DrawTime` 10000.0))
  (bind (_bblockinghit _binitialoverlap _time _distance _location _impactpoint _normal _impactnormal _physmat _hitactor _hitcomponent _hitbonename _bonename _hititem _elementindex _faceindex _tracestart _traceend) (`GameplayStatics.BreakHitResult` _outhit))
  (return (`KismetMathLibrary.SelectVector` _location _traceend _returnvalue_2)))

(fn `LanchPorjectile`
  (bind _fireprojectile (`self.FireProjectile`))
  (bind _fireprojectile_2 (`self.FireProjectile`))
  (bind _projectilemovement (`BaseProjectile.ProjectileMovement` _fireprojectile_2))
  (`/Engine/EditorBlueprintResources/StandardMacros.IsValid` (`self.FireProjectile`)
    (:`Is Valid`
      (bind _returnvalue (`self.ShootLineBone` 5000.0))
      (`self.K2_DetachFromActor` _fireprojectile "KeepRelative" "KeepRelative" "KeepRelative")
      (`self.K2_SetActorTransform` _fireprojectile _returnvalue false false)
      (set `ProjectileMovementComponent.bSimulationEnabled` true _projectilemovement)
      (set `MovementComponent.Velocity` (* (`SceneComponent.GetForwardVector` (`BaseProjectile.StaticMesh` _fireprojectile_2)) (`WeaponData.ProjectileSpeed` (`self.DataAsset`))) _projectilemovement))))

(fn `ShootLineBone`
  (params (TraceRange :type "Float (double-precision)"))
  (returns (ReturnValue :type "Transform Structure"))
  (bind _location (.location (`SceneComponent.GetSocketTransform` (`self.SkeletalMesh`) "None" "RTS_World")))
  (bind _returnvalue (`self.CameraLineTrace` TraceRange))
  (return (`KismetMathLibrary.MakeTransform` _location (`KismetMathLibrary.FindLookAtRotation` _location _returnvalue))))

(fn `SpawnProjectile`
  (bind _projectileclass (`WeaponData.ProjectileClass` (`self.DataAsset`)))
  (if (`KismetSystemLibrary.IsValidClass` _projectileclass)
    (bind _returnvalue (`|SpawnActorFromClass` _projectileclass (`KismetMathLibrary.MakeTransform` (0.0 0.0 0.0)) "Undefined" "MultiplyWithRoot" null null))
    (bind _output_get (set `self.FireProjectile` _returnvalue))
    (set `ProjectileMovementComponent.InitialSpeed` (`WeaponData.ProjectileSpeed` (`self.DataAsset`)) (`BaseProjectile.ProjectileMovement` _output_get))
    (`self.K2_AttachToComponent` _output_get (`self.SkeletalMesh`) "ArrowSocket" "KeepRelative" "KeepRelative" "KeepRelative" true)))

(fn `UserConstructionScript`)