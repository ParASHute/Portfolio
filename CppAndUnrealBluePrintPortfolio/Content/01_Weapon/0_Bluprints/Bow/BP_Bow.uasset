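; Bow weapon Blueprint that provides functions to nock and fire arrows for its owning character.
; SpawnProjectile creates the DataAsset's projectile with collision off on the mesh's ArrowSocket, an attach point noted as provisional until the character AnimBP is finished.
; LanchPorjectile restores capsule overlap, detaches the arrow and launches it along control rotation at DataAsset speed.
; HoldCamera locks or unlocks the owner's camera from the Attack.DrawingBow gameplay tag.
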(event `self.ReceiveBeginPlay`)

(fn `HoldCamera`
  (bind _returnvalue (> (`AbilitySystemComponent.GetGameplayTagCount` (`AbilitySystemBlueprintLibrary.GetAbilitySystemComponent` (`self.OwnerCharacter`)) (struct :`TagName` "Attack.DrawingBow")) 0))
  (if _returnvalue
    (`PortfolioCharacter.CameraLock` (`self.OwnerCharacter`) _returnvalue)
    (else
      (`PortfolioCharacter.CameraUnLock` (`self.OwnerCharacter`) _returnvalue))))

(fn `LanchPorjectile`
  (bind _projectilemovement (`BaseProjectile.ProjectileMovement` (`self.FireProjectile`)))
  (`PrimitiveComponent.SetCollisionProfileName` (`BaseProjectile.Capsule` (`self.FireProjectile`)) "OverlapAllDynamic" true)
  (`/Engine/EditorBlueprintResources/StandardMacros.IsValid` (`self.FireProjectile`)
    (:`Is Valid`
      (`self.K2_DetachFromActor` (`self.FireProjectile`) "KeepWorld" "KeepWorld" "KeepWorld")
      (set `ProjectileMovementComponent.bSimulationEnabled` true _projectilemovement)
      (set `MovementComponent.Velocity` (* (`KismetMathLibrary.GetForwardVector` (`Pawn.GetControlRotation` (`self.OwnerCharacter`))) (`WeaponData.ProjectileSpeed` (`self.DataAsset`))) _projectilemovement))))

(fn `SpawnProjectile`
  (bind _projectileclass (`WeaponData.ProjectileClass` (`self.DataAsset`)))
  (if (`KismetSystemLibrary.IsValidClass` _projectileclass)
    (bind _returnvalue (`|SpawnActorFromClass` _projectileclass (`KismetMathLibrary.MakeTransform` (0.0 0.0 0.0)) "Undefined" "MultiplyWithRoot" null (`self.OwnerCharacter`)))
    (bind _output_get (set `self.FireProjectile` _returnvalue))
    (`PrimitiveComponent.SetCollisionProfileName` (`BaseProjectile.StaticMesh` _output_get) "NoCollision" true)
    (`PrimitiveComponent.SetCollisionProfileName` (`BaseProjectile.Capsule` _output_get) "NoCollision" true)
    (set `ProjectileMovementComponent.InitialSpeed` (`WeaponData.ProjectileSpeed` (`self.DataAsset`)) (`BaseProjectile.ProjectileMovement` _output_get))
    (`self.K2_AttachToComponent` _output_get (`self.SkeletalMesh`) "ArrowSocket" "KeepRelative" "KeepRelative" "KeepRelative" true)))

(fn `UserConstructionScript`)