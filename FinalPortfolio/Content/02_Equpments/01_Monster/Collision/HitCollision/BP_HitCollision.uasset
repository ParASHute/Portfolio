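; BP_HitCollision is a monster hit-detection Blueprint that sphere-traces between two points for Bokoblin attacks.
; CreateMultiSphere spawns an impact emitter via a channel trace, then runs a single-result object trace.
; On an object hit, a Bokoblin owner receives a Hit gameplay event and deals fixed damage, ignoring the stored Damage; any other owner makes it destroy itself.
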(event `CreateFX`
  (params (EmitterTemplate :type "ParticleSystem Object Reference") (Location :type "Vector Structure"))
  (`GameplayStatics.SpawnEmitterAtLocation` EmitterTemplate Location))

(fn `CreateMultiSphere`
  (params (StartPoint :type "Vector Structure") (EndPoint :type "Vector Structure") (Radius :type "Float (double-precision)"))
  (returns (Hit :type Boolean))
  (locals (NewLocalVar :type Boolean :default false))
  (`self.CreatHitFX` StartPoint EndPoint Radius)
  (bind (_outhit _returnvalue) (`KismetSystemLibrary.SphereTraceSingleForObjects` StartPoint EndPoint Radius (`|MakeArray` "ObjectTypeQuery8" :!type "EObjectTypeQuery Enum") false (`|MakeArray` (`self.GetOwner`)) "None" true (struct :`R` 1.0 :`A` 1.0) (struct :`G` 1.0 :`A` 1.0) 10000.0))
  (if _returnvalue
    (set `local.NewLocalVar` true)
    (bind _asbp_base_bokoblin (cast `/Game/03_Characters/01_AI/BP_BaseBokoblin` (`self.GetOwner`))
      (:`then`
        (bind (_bblockinghit _binitialoverlap _time _distance _location _impactpoint _normal _impactnormal _physmat _hitactor) (`GameplayStatics.BreakHitResult` _outhit))
        (`AbilitySystemBlueprintLibrary.SendGameplayEventToActor` _asbp_base_bokoblin (struct :`TagName` "Hit") (make `GameplayEventData` (struct) null _hitactor))
        (`GameplayStatics.ApplyDamage` _hitactor 1.0 null _asbp_base_bokoblin)
        (return (`local.NewLocalVar`)))
      (:`CastFailed`
        (`self.K2_DestroyActor`)))))

(fn `CreatHitFX`
  (params (StartPoint :type "Vector Structure") (EndPoint :type "Vector Structure") (Radius :type "Float (double-precision)"))
  (bind _emitter_template (`self.Emitter Template`))
  (set `self.HitPoint` EndPoint)
  (bind (_outhit _returnvalue) (`KismetSystemLibrary.SphereTraceSingle` StartPoint EndPoint Radius "TraceTypeQuery4" false (`|MakeArray` (`self.GetOwner`))))
  (if _returnvalue
    (bind (_bblockinghit _binitialoverlap _time _distance _location _impactpoint _normal _impactnormal _physmat _hitactor) (`GameplayStatics.BreakHitResult` _outhit))
    (set `self.HitPoint` _location)
    (cast `/Game/03_Characters/BP_BaseCharacter` _hitactor
      (:`then`
        (`self.CreateFX` _emitter_template _location))
      (:`CastFailed`
        (`self.CreateFX` _emitter_template _location)))))

(fn `OnInit`
  (params (Radius :type "Float (double-precision)") (Damage :type "Float (double-precision)"))
  (set `self.Radius` Radius)
  (set `self.Damage` Damage))

(fn `UserConstructionScript`)