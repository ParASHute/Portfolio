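; Base character Blueprint that handles damage reactions and death cleanup.
; On BeginPlay it makes mesh materials dynamic so damage can briefly flash them red.
; While a Gameplay Ability System attribute is positive, damage also temporarily swaps the collision object type, derives the armed weapon from gameplay tags and plays a directional or shield hit montage.
; MakeDeath disables collision and destroys the actor after a delay.
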(event `self.ReceiveBeginPlay`
  ;[1 1 1] 매쉬의 색을 수정하기 위한 작업
  (for (_array_element _array_index) (`MeshComponent.GetMaterials` (`self.Mesh`))
    (bind _returnvalue (`KismetMaterialLibrary.CreateDynamicMaterialInstance` _array_element "None" "Transient"))
    (`PrimitiveComponent.SetMaterial` (`self.Mesh`) _array_index _returnvalue)))

(event `self.ReceiveAnyDamage`
  (params (Damage :type "Float (single-precision)") (DamageType :type "DamageType Object Reference") (InstigatedBy :type "Controller Object Reference") (DamageCauser :type "Actor Object Reference"))
  (bind _abilitysystemcomponent (`self.AbilitySystemComponent`))
  (bind (_sheild_hit_montage_montage _sheild_hit_montage_playrate) (break `Montage` (`self.Sheild Hit Montage`)))
  (bind _hitmontage (`self.HitMontage`))
  (bind _collision (`self.Collision`))
  (bind _returnvalue (`MeshComponent.GetMaterials` (`self.Mesh`)))
  (bind (_output_montage _output_playrate) (break `Montage` (`|GetArrayItem` _hitmontage (`WeaponComponent.FindCaurserDirection` (`self.WeaponComponent`) DamageCauser _hitmontage))))
  ;[1 1 1] 데미지를 받았을때 수행할 작업들
  ; 죽었을땐 각각 따로 실행
  (set `self.DamageCurser` DamageCauser)
  (if (> (`.ReturnValue` (`AbilitySystemComponent.GetGameplayAttributeValue` (`self.AbilitySystemComponent`) (struct :`AttributeName` "CurrentHealth" :`Attribute` "/Script/Portfolio.MyAttributeSet:CurrentHealth" :`AttributeOwner` "/Script/CoreUObject.Class'/Script/Portfolio.MyAttributeSet'"))) 0.0)
    (`|ExecutionSequence`
      (:`then_0`
        (set `self.ObjType` (`PrimitiveComponent.GetCollisionObjectType` _collision))
        (`PrimitiveComponent.SetCollisionObjectType` _collision "ECC_GameTraceChannel5")
        (`KismetSystemLibrary.Delay` 0.1)
        (`PrimitiveComponent.SetCollisionObjectType` (`self.Collision`) (`self.ObjType`)))
      (:`then_1`
        (for _array_element _returnvalue
          (bind `_as머티리얼_인스턴스_다이내믹` (cast `MaterialInstanceDynamic` _array_element))
          (`MaterialInstanceDynamic.SetVectorParameterValue` `_as머티리얼_인스턴스_다이내믹` "Color" (struct :`R` 1.0 :`A` 1.0)))
        (`KismetSystemLibrary.Delay` 0.5)
        (for _array_element_2 _returnvalue
          (bind `_as머티리얼_인스턴스_다이내믹_2` (cast `MaterialInstanceDynamic` _array_element_2))
          (`MaterialInstanceDynamic.SetVectorParameterValue` `_as머티리얼_인스턴스_다이내믹_2` "Color" (struct :`R` 1.0 :`G` 1.0 :`B` 1.0 :`A` 1.0))))
      (:`then_2`
        (if (> (`AbilitySystemComponent.GetGameplayTagCount` _abilitysystemcomponent (struct :`TagName` "Defence.Idle")) 0)
          (set `self.ArmdWeapon` "Shield")
          (elif (> (`AbilitySystemComponent.GetGameplayTagCount` _abilitysystemcomponent (struct :`TagName` "State.ArmdSwrod")) 0)
            (set `self.ArmdWeapon` "Sword")
            (elif (> (`AbilitySystemComponent.GetGameplayTagCount` _abilitysystemcomponent (struct :`TagName` "State.ArmdBow")) 0)
              (set `self.ArmdWeapon` "Bow")
              (else
                (set `self.ArmdWeapon` "None"))))))
      (:`then_3`
        (switch `EWeaponType` (`self.ArmdWeapon`)
          (:`None`
            (`/Engine/EditorBlueprintResources/StandardMacros.IsValid` _output_montage :!label _label
              (:`Is Valid`
                (`self.PlayAnimMontage` _output_montage _output_playrate))))
          (:`Sword`
            (goto _label))
          (:`Bow`
            (goto _label))
          (:`Shield`
            (if (!= (`WeaponComponent.FindCaurserDirection` (`self.WeaponComponent`) DamageCauser (`|MakeArray` (`self.Sheild Hit Montage`))) 2)
              (`/Engine/EditorBlueprintResources/StandardMacros.IsValid` _sheild_hit_montage_montage
                (:`Is Valid`
                  (`self.PlayAnimMontage` _sheild_hit_montage_montage _sheild_hit_montage_playrate))))))))))

(event `MakeDeath`
  (`PrimitiveComponent.SetCollisionEnabled` (`self.CapsuleComponent`) "NoCollision")
  (`PrimitiveComponent.SetCollisionEnabled` (`self.Collision`) "NoCollision")
  (`KismetSystemLibrary.Delay` 1.5)
  (`self.K2_DestroyActor`))

(fn `UserConstructionScript`)