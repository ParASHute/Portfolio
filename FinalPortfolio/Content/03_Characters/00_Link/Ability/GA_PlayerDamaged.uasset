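; GA_PlayerDamaged is a gameplay ability that handles damage taken by the player character Link.
; Once committed, it listens for a single Hit.Hit3 gameplay event and applies GE_Damage to the payload's target, passing the event magnitude via SetByCaller.
; After a short delay, it clears the Swapping flag on BP_Link's WeaponComponent and ends, so the listening window is brief.
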(event `self.K2_ActivateAbility`
  (bind _returnvalue (`self.K2_CommitAbility`))
  (if _returnvalue
    (bind (_asynctaskproxy _payload) (`AbilityTask_WaitGameplayEvent.WaitGameplayEvent` (struct :`TagName` "Hit.Hit3") null true)
      (:`then`
        _)
      (:`EventReceived`
        (bind (_eventtag _instigator _target _optionalobject _optionalobject2 _contexthandle _instigatortags _targettags _eventmagnitude) (break `GameplayEventData` _payload))
        (bind _returnvalue_2 (`AbilitySystemBlueprintLibrary.GetAbilitySystemComponent` _target))
        (bind _returnvalue_3 (`AbilitySystemBlueprintLibrary.AssignTagSetByCallerMagnitude` (`AbilitySystemComponent.MakeOutgoingSpec` :`self` _returnvalue_2 :`GameplayEffectClass` "/Game/03_Characters/00_Link/Ability/GE_Damage.GE_Damage_C" :`Level` 1.0) (struct :`TagName` "Hit.Hit3") _eventmagnitude))
        (`AbilitySystemComponent.BP_ApplyGameplayEffectSpecToSelf` _returnvalue_2 _returnvalue_3)))
    (`KismetSystemLibrary.Delay` 0.25)
    (bind _asbp_link (cast `/Game/03_Characters/00_Link/BP_Link` (`self.GetOwningActorFromActorInfo`)))
    (set `WeaponComponent.Swapping` false (`PortfolioCharacter.WeaponComponent` _asbp_link))
    (`self.K2_EndAbility`)))