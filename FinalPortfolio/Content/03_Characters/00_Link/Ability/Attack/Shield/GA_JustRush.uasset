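; Link's backward dodge gameplay ability, which can trigger a "Just Rush" window on a well-timed evade.
; It plays a sped-up dodge montage while a constant root-motion force pushes Link backward.
; A Monster.State.CanParry event during the dodge starts Just Rush time on Link and sends JustRushTime to his target.
; On blend out it reactivates Defence unless cancelled, then ends; interruption or cancellation just ends it.
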(event `self.K2_ActivateAbility`
  (bind _link (`self.Link`))
  (bind _returnvalue (`self.K2_CommitAbility`))
  (if _returnvalue
    (`AbilityTask_PlayMontageAndWait.CreatePlayMontageAndWaitProxy` "None" "/Game/00_PlayerAnimation/02_Montage/02_Shield/Dodge/IP_dodge_back_Montage.IP_dodge_back_Montage" 2.0
      (:`then`
        (bind _asbp_link (cast `/Game/03_Characters/00_Link/BP_Link` (`self.GetOwningActorFromActorInfo`)))
        (bind _output_get (set `self.Link` _asbp_link))
        (`AbilityTask_ApplyRootMotionConstantForce.ApplyRootMotionConstantForce` "None" (* (`Actor.GetActorForwardVector` _output_get) -1.0) 150.0 0.8 false null "MaintainLastRootMotionVelocity" (`Actor.GetVelocity` _asbp_link)
          (:`then`
            (`AbilityTask_WaitGameplayEvent.WaitGameplayEvent` (struct :`TagName` "Monster.State.CanParry") null true
              (:`EventReceived`
                (`/Game/03_Characters/00_Link/BP_Link.SetJustRushTime` _link)
                (`AbilitySystemBlueprintLibrary.SendGameplayEventToActor` (`/Game/03_Characters/00_Link/BP_Link.TargetActor` _link) (struct :`TagName` "Monster.State.JustRushTime")))))))
      (:`OnBlendOut`
        (bind _asbp_link_2 (cast `/Game/03_Characters/00_Link/BP_Link` (`self.GetOwningActorFromActorInfo`)))
        (if (not (`/Game/03_Characters/00_Link/BP_Link.Cancled` _asbp_link_2))
          (`AbilitySystemComponent.TryActivateAbilitiesByTag` (`PortfolioCharacter.AbilitySystemComponent` _asbp_link_2) (`BlueprintGameplayTagLibrary.MakeLiteralGameplayTagContainer` (struct :`GameplayTags` (struct :`(TagName` "State.Defence")))) true))
        (`self.K2_EndAbility`))
      (:`OnInterrupted`
        (`self.K2_EndAbility` :!label _label))
      (:`OnCancelled`
        (goto _label)))
    (else
      (`self.K2_EndAbility`))))