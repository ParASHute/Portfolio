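; GA_ShootArrow is a gameplay ability that makes Link fire an arrow from his equipped bow.
; On activation it commits the ability, casts the owning actor to BP_Link and takes the current weapon from its WeaponComponent as BP_Bow.
; It then calls the bow's projectile launch and ends at once, also ending when the commit fails.
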(event `self.K2_ActivateAbility`
  (bind _returnvalue (`self.K2_CommitAbility`))
  (if _returnvalue
    (bind _asbp_link (cast `/Game/03_Characters/00_Link/BP_Link` (`self.GetOwningActorFromActorInfo`)))
    (bind _asbp_bow (cast `/Game/02_Equpments/0_WeaponBluprints/01_Bow/BP_Bow` (`WeaponComponent.CurrentWeapon` (`PortfolioCharacter.WeaponComponent` _asbp_link))))
    (`/Game/02_Equpments/0_WeaponBluprints/01_Bow/BP_Bow.LanchPorjectile` _asbp_bow)
    (`self.K2_EndAbility`)
    (else
      (`self.K2_EndAbility`))))