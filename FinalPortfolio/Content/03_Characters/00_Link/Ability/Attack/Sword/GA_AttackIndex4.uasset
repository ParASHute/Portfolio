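; GA_AttackIndex4 is a gameplay ability for Link's sword attack index 4.
; It commits, sets the weapon component's Swapping flag, and plays the Attack_04 montage.
; A Hit.Hit1 gameplay event applies GE_Damage to its target, using SetByCaller magnitude scaled negatively from current weapon damage.
; All montage exits end the ability, but only Completed clears Swapping.
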(event `self.K2_ActivateAbility`
  (bind _returnvalue (`self.K2_CommitAbility`))
  (if _returnvalue
    (bind _asbp_link (cast `/Game/03_Characters/00_Link/BP_Link` (`self.GetOwningActorFromActorInfo`)))
    (bind _output_get (set `self.As BP Link` _asbp_link))
    (set `WeaponComponent.Swapping` true (`PortfolioCharacter.WeaponComponent` _output_get))
    (`AbilityTask_PlayMontageAndWait.CreatePlayMontageAndWaitProxy` "None" "/Game/00_PlayerAnimation/02_Montage/00_Sword/Attack/Attack_04_Seq_Montage.Attack_04_Seq_Montage"
      (:`then`
        (bind (_asynctaskproxy _payload) (`AbilityTask_WaitGameplayEvent.WaitGameplayEvent` (struct :`TagName` "Hit.Hit1") null) ; 테그 이벤트 발송시 뒤에것들 실행
          (:`EventReceived`
            (bind _returnvalue_2 (`AbilitySystemBlueprintLibrary.AssignTagSetByCallerMagnitude` (`self.MakeOutgoingGameplayEffectSpec` "/Game/03_Characters/00_Link/Ability/GE_Damage.GE_Damage_C") (struct :`TagName` "Hit.Hit1") (* (`WeaponData.WeaponDamage` (`WeaponComponent.CurrentWeaponDataAsset` (`PortfolioCharacter.WeaponComponent` (`self.As BP Link`)))) -0.75)))
            (`AbilitySystemComponent.BP_ApplyGameplayEffectSpecToSelf` (`AbilitySystemBlueprintLibrary.GetAbilitySystemComponent` (`.Target` (break `GameplayEventData` _payload))) _returnvalue_2))))
      (:`OnCompleted`
        (set `WeaponComponent.Swapping` false (`PortfolioCharacter.WeaponComponent` (`self.As BP Link`)))
        (`self.K2_EndAbility`))
      (:`OnBlendOut`
        (`self.K2_EndAbility` :!label _label))
      (:`OnInterrupted`
        (goto _label))
      (:`OnCancelled`
        (goto _label)))
    (else
      (`self.K2_EndAbility`))))