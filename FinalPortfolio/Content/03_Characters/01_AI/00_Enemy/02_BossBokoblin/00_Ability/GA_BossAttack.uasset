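; Gameplay Ability for the boss Bokoblin's melee attack, played through the Troll_Attack_1 montage.
; A Monster.Boss.Attack event on the owner triggers a server-only MeleeAttack unless the JustRushTime state tag is present.
; A one-shot Hit event listener applies GE_Damage to the payload target, passing Damage as a SetByCaller magnitude.
; The ability ends on montage blend-out, interruption, cancellation or failed commit.
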(event `self.K2_ActivateAbility`
  (bind _returnvalue (`self.GetOwningActorFromActorInfo`))
  (bind _returnvalue_2 (`self.K2_CommitAbility`))
  (if _returnvalue_2
    (`AbilityTask_PlayMontageAndWait.CreatePlayMontageAndWaitProxy` "None" "/Game/01_MonsterAnimation/03_Montage/Boss/Attack/Troll_Attack_1.Troll_Attack_1"
      (:`then`
        (`AbilityAsync_WaitGameplayEvent.WaitGameplayEventToActor` _returnvalue (struct :`TagName` "Monster.Boss.Attack")
          (:`then`
            (bind (_asynctaskproxy _payload) (`AbilityTask_WaitGameplayEvent.WaitGameplayEvent` (struct :`TagName` "Hit") null true)
              (:`EventReceived`
                (bind _returnvalue_3 (`AbilitySystemBlueprintLibrary.GetAbilitySystemComponent` (`.Target` (break `GameplayEventData` _payload))))
                (bind _returnvalue_4 (`AbilitySystemBlueprintLibrary.AssignTagSetByCallerMagnitude` (`AbilitySystemComponent.MakeOutgoingSpec` :`self` _returnvalue_3 :`GameplayEffectClass` "/Game/03_Characters/00_Link/Ability/GE_Damage.GE_Damage_C" :`Level` 1.0) (struct :`TagName` "Hit.Hit1") (`self.Damage`)))
                (`AbilitySystemComponent.BP_ApplyGameplayEffectSpecToSelf` _returnvalue_3 _returnvalue_4))))
          (:`EventReceived`
            (`self.K2_HasAuthority`
              (:`True`
                (if (< (`AbilitySystemComponent.GetGameplayTagCount` (`AbilitySystemBlueprintLibrary.GetAbilitySystemComponent` _returnvalue) (struct :`TagName` "Monster.State.JustRushTime")) 1)
                  (`self.MeleeAttack` 200.0)))))))
      (:`OnBlendOut`
        (`self.K2_EndAbility` :!label _label))
      (:`OnInterrupted`
        (goto _label))
      (:`OnCancelled`
        (goto _label)))
    (else
      (`self.K2_EndAbility`))))